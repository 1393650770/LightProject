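; Anim notify that shows or hides the bow's arrow and sets whether it attaches to the hand or the bow during an animation.
; On trigger it gets the displayed item from the mesh owner's EquipmentComponent, casts it to DI_Bow, and passes on the AttachToHand and Visible settings.
; The notify name is built from both settings, so it describes the resulting arrow state.
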(fn `GetNotifyName`
  (returns (ReturnValue :type String))
  (return (`KismetStringLibrary.Concat_StrStr` (select `bool` (`self.Visible`) :`false` "Hide" :`true` "Show") " Arrow" (select `bool` (`self.Visible`) :`true` (`KismetStringLibrary.Concat_StrStr` " and attach to " (select `bool` (`self.AttachToHand`) :`false` "Bow" :`true` "Hand"))))))

(fn `Received_Notify`
  (params (MeshComp :type "SkeletalMeshComponent Object Reference") (Animation :type "AnimSequenceBase Object Reference"))
  (returns (ReturnValue :type Boolean))
  (bind _returnvalue (`ActorComponent.GetOwner` MeshComp))
  (bind _returnvalue_2 (`Actor.GetComponentByClass` _returnvalue "/Game/DynamicCombatSystem/Blueprints/Components/EquipmentComponent.EquipmentComponent_C"))
  (bind _displayeditem (`/Game/DynamicCombatSystem/Blueprints/Components/EquipmentComponent.GetDisplayedItem` _returnvalue_2 "NewEnumerator19" 0))
  (`/Engine/EditorBlueprintResources/StandardMacros.IsValid` _returnvalue
    (:`Is Valid`
      (`/Engine/EditorBlueprintResources/StandardMacros.IsValid` _returnvalue_2
        (:`Is Valid`
          (`/Engine/EditorBlueprintResources/StandardMacros.IsValid` _displayeditem
            (:`Is Valid`
              (bind _asdi_bow (cast `/Game/DynamicCombatSystem/Blueprints/Items/DisplayedItems/DI_Bow` _displayeditem))
              (`/Game/DynamicCombatSystem/Blueprints/Items/DisplayedItems/DI_Bow.UpdateArrowAttachment` _asdi_bow (`self.AttachToHand`))
              (`/Game/DynamicCombatSystem/Blueprints/Items/DisplayedItems/DI_Bow.UpdateArrowVisibility` _asdi_bow (`self.Visible`))
              (return false))))))))